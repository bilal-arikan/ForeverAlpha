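; BP_Shield is a shield actor that absorbs BP_Ammo projectiles, making them explode on overlap or hit.
; Each absorb shows the sphere and plays a timeline that drives a brightness parameter on its material, then hides the sphere when finished.
; The construction script creates that dynamic material instance, assigns it to the sphere and sets the default brightness.
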(event `self.ReceiveBeginPlay`)

(event `self.ReceiveActorBeginOverlap`
  (params (OtherActor :type "Actor Object Reference")))

(event `self.ReceiveTick`
  (params (DeltaSeconds :type "Float (single-precision)")))

(event `self.ReceiveActorBeginOverlap`
  (params (OtherActor :type "Actor Object Reference"))
  (bind _as_bp_ammo (cast `/Game/Editor/ShipModuls/Ammo/_BP_Ammo` OtherActor))
  (`self.Absorb`)
  (`/Game/Editor/ShipModuls/Ammo/_BP_Ammo.Explode` _as_bp_ammo))

(event `self.ReceiveHit`
  (params (MyComp :type "PrimitiveComponent Object Reference") (Other :type "Actor Object Reference") (OtherComp :type "PrimitiveComponent Object Reference") (bSelfMoved :type Boolean) (HitLocation :type "Vector Structure") (HitNormal :type "Vector Structure") (NormalImpulse :type "Vector Structure") (Hit :type "HitResult Structure (by ref)"))
  (bind _as_bp_ammo (cast `/Game/Editor/ShipModuls/Ammo/_BP_Ammo` Other))
  (`self.Absorb`)
  (`/Game/Editor/ShipModuls/Ammo/_BP_Ammo.Explode` _as_bp_ammo))

(event `Absorb`
  (`SceneComponent.SetVisibility` (`self.Sphere`) true false)
  (bind (_direction _newtrack_0) (`Timeline|Timeline_0` :!via `PlayFromStart` :!label _label)
    (:`Update`
      (`MaterialInstanceDynamic.SetScalarParameterValue` (`self.DynamicMaterialInst`) (`self.Name_Brightness`) (* _newtrack_0 10.0)))
    (:`Finished`
      (`SceneComponent.SetVisibility` (`self.Sphere`) false false)
      (goto _label :!via `SetNewTime`))))

(fn `UserConstructionScript`
  (bind _returnvalue (`KismetMaterialLibrary.CreateDynamicMaterialInstance` (`self.Material`)))
  (bind _output_get (set `self.DynamicMaterialInst` _returnvalue))
  (`PrimitiveComponent.SetMaterial` (`self.Sphere`) 0 _output_get)
  (`MaterialInstanceDynamic.SetScalarParameterValue` (`self.DynamicMaterialInst`) (`self.Name_Brightness`) (`self.DefaultBrightness`)))