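; BP_SpaceBox is a space backdrop actor from the SpaceScapes assets, built on a single static mesh with six material slots.
; The construction script assigns six material variables to the mesh's slots, one per slot, so the box's look follows those variables.
; It has no runtime logic, as the event graph holds only disabled placeholder events.
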(event `self.ReceiveBeginPlay`)

(event `self.ReceiveActorBeginOverlap`
  (params (OtherActor :type "Actor Object Reference")))

(event `self.ReceiveTick`
  (params (DeltaSeconds :type "Float (single-precision)")))

(fn `UserConstructionScript`
  (bind _staticmesh (`self.StaticMesh`))
  (`PrimitiveComponent.SetMaterial` _staticmesh 0 (`self.Material_0`))
  (`PrimitiveComponent.SetMaterial` _staticmesh 1 (`self.Material_1`))
  (`PrimitiveComponent.SetMaterial` _staticmesh 2 (`self.Material_2`))
  (`PrimitiveComponent.SetMaterial` _staticmesh 3 (`self.Material_3`))
  (`PrimitiveComponent.SetMaterial` _staticmesh 4 (`self.Material_4`))
  (`PrimitiveComponent.SetMaterial` _staticmesh 5 (`self.Material_5`)))