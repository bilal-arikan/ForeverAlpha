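; BP_AsteroidCloud is an actor that fills a volume around itself with randomly scattered asteroids.
; Its Construction Script loops on Count, adding child actor components of the Asteroid class, each with a random rotation and non-uniform random scale.
; The Sphere component's radius, multiplied by ten, sets the half-extent of the scatter, so the cloud is cubic rather than spherical.
; The event graph has no active logic.
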(fn `UserConstructionScript`
  (bind _returnvalue (`KismetMathLibrary.RandomFloatInRange` 0.5 1.0))
  (bind _returnvalue_2 (* (`SphereComponent.SphereRadius` (`self.Sphere`)) 10.0))
  (bind _returnvalue_3 (* _returnvalue_2 -1.0))
  (for _ (range (+ (`self.Count`) 1))
    (bind _returnvalue_4 (`AddComponent|NODE_AddChildActorComponent-0` :`RelativeTransform` (`KismetMathLibrary.MakeTransform` (`KismetMathLibrary.MakeVector` (`KismetMathLibrary.RandomFloatInRange` _returnvalue_3 _returnvalue_2) (`KismetMathLibrary.RandomFloatInRange` _returnvalue_3 _returnvalue_2) (`KismetMathLibrary.RandomFloatInRange` _returnvalue_3 _returnvalue_2)) (`KismetMathLibrary.RandomRotator` true) (`KismetMathLibrary.MakeVector` _returnvalue _returnvalue _returnvalue))))
    (`ChildActorComponent.SetChildActorClass` _returnvalue_4 "/Game/Editor/Assets/Asteroids/Asteroid.Asteroid_C")))