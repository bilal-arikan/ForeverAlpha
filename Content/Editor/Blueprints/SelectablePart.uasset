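; Base actor for spaceship parts and modules, forming a parent-child attachment tree for ship building.
; Selection swaps materials and hover toggles custom depth for highlighting.
; Depleted health recursively deletes modules and drops parts as physics bodies, destroying the ship for Part_Main, while manual deletion destroys the whole branch.
; GetAllSStructs recursively flattens the tree into ID-tagged design structs, and MakeSelectable spawns an actor from one.
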(event `AttachLikeModul`
  (params (ChildModul :type "/Game/Editor/Blueprints/SelectablePart Object Reference"))
  (`/Engine/EditorBlueprintResources/StandardMacros.IsValid` ChildModul
    (:`Is Valid`
      (set `/Game/Editor/Blueprints/SelectablePart.ParentPart` self ChildModul)
      (set `/Game/Editor/Blueprints/SelectablePart.SpaceShipRef` (`self.SpaceShipRef`) ChildModul)
      (`SceneComponent.K2_AttachTo` (`/Game/Editor/Blueprints/SelectablePart.StaticMesh` ChildModul) (`self.StaticMesh`) "None" "KeepWorldPosition" true)
      (`KismetArrayLibrary.Array_Add` (`self.ConnectedModuls`) ChildModul))))

(event `AttachLikePart`
  (params (ChildPart :type "/Game/Editor/Blueprints/SelectablePart Object Reference"))
  (`/Engine/EditorBlueprintResources/StandardMacros.IsValid` ChildPart
    (:`Is Valid`
      (set `/Game/Editor/Blueprints/SelectablePart.ParentPart` self ChildPart)
      (set `/Game/Editor/Blueprints/SelectablePart.SpaceShipRef` (`self.SpaceShipRef`) ChildPart)
      (`SceneComponent.K2_AttachTo` (`/Game/Editor/Blueprints/SelectablePart.StaticMesh` ChildPart) (`self.StaticMesh`) "None" "KeepWorldPosition" true)
      (`KismetArrayLibrary.Array_Add` (`self.ConnectedParts`) ChildPart))))

(event `DeleteModuls`
  (for _array_element (`self.ConnectedModuls`)
    (`self.Delete` _array_element))
  (`KismetArrayLibrary.Array_Clear` (`self.ConnectedModuls`)))

(event `Delete`
  (`self.DeleteFunc`))

(event `Select`
  (if (`self.isSelected`)
    (set `self.isSelectedTwice` true)
    (else
      (set `self.isSelectedTwice` false)
      (set `self.isSelected` true)
      (`PrimitiveComponent.SetMaterial` (`self.StaticMesh`) 0 (`self.MaterialSelected`)))))

(event `CursorHover`
  (set `self.isCursorHovered` true)
  (`PrimitiveComponent.SetRenderCustomDepth` (`self.StaticMesh`) true))

(event `CursorUnhover`
  (set `self.isCursorHovered` false)
  (`PrimitiveComponent.SetRenderCustomDepth` (`self.StaticMesh`) false))

(event `Unselect`
  (if (`self.isSelected`)
    _
    (else
      _))
  (set `self.isSelectedTwice` false)
  (set `self.isSelected` false)
  (`PrimitiveComponent.SetMaterial` (`self.StaticMesh`) 0 (`self.MaterialDefault`)))

(event `self.ReceiveActorBeginOverlap`
  (params (OtherActor :type "Actor Object Reference"))
  (set `self.isOverlapped` true))

(event `self.ReceiveActorEndOverlap`
  (params (OtherActor :type "Actor Object Reference"))
  (set `self.isOverlapped` false))

(event `TakeDamage`
  (params (damageValue :type "Float (double-precision)"))
  (bind _output_get (set `self.Health` (- (`self.Health`) damageValue)))
  (if (> 0.0 _output_get)
    (`self.DestroyWithDamage`)))

(event `Simulate`
  (params (isSimulating :type Boolean))
  (bind _textid (`self.TextID`))
  (if isSimulating
    (`SceneComponent.SetVisibility` _textid false false)
    (for _array_element (`self.ConnectedModuls`)
      (`self.Simulate` _array_element true))
    (set `self.isSimulating` true)
    (else
      (`SceneComponent.SetVisibility` _textid true false)
      (for _array_element_2 (`self.ConnectedModuls`)
        (`self.Simulate` _array_element_2 false))
      (set `self.isSimulating` false))))

(fn `DeleteFunc`
  (bind _parentpart (`self.ParentPart`))
  (bind _connectedparts (`self.ConnectedParts`))
  (bind _connectedmoduls (`self.ConnectedModuls`))
  (bind _returnvalue (> (`KismetArrayLibrary.Array_Length` _connectedmoduls) 0))
  (bind _returnvalue_2 (> (`KismetArrayLibrary.Array_Length` _connectedparts) 0))
  (if _returnvalue
    (`self.DeleteFunc` (`KismetArrayLibrary.Array_Get` _connectedmoduls) :!label _label)
    (if _returnvalue
      (goto _label)
      (else
        _)))
  (if _returnvalue_2
    (`self.DeleteFunc` (`KismetArrayLibrary.Array_Get` _connectedparts) :!label _label_2)
    (if _returnvalue_2
      (goto _label_2)
      (else
        _)))
  (`/Engine/EditorBlueprintResources/StandardMacros.IsValid` _parentpart
    (:`Is Valid`
      (`KismetArrayLibrary.Array_RemoveItem` (`/Game/Editor/Blueprints/SelectablePart.ConnectedParts` _parentpart) self)
      (`KismetArrayLibrary.Array_RemoveItem` (`/Game/Editor/Blueprints/SelectablePart.ConnectedModuls` _parentpart) self))
    (:`Is Not Valid`
      _))
  (`self.K2_DestroyActor`))

(fn `DestroyWithDamage`
  (bind _connectedparts (`self.ConnectedParts`))
  (bind _connectedmoduls (`self.ConnectedModuls`))
  (bind _parentpart (`self.ParentPart`))
  (bind _spaceshipref (`self.SpaceShipRef`))
  (bind _returnvalue (> (`KismetArrayLibrary.Array_Length` _connectedmoduls) 0))
  (bind _returnvalue_2 (> (`KismetArrayLibrary.Array_Length` _connectedparts) 0))
  (`/Engine/EditorBlueprintResources/StandardMacros.IsValid` (`self.SpaceShipRef`)
    (:`Is Valid`
      (if _returnvalue
        (`self.Delete` (`KismetArrayLibrary.Array_Get` _connectedmoduls) :!label _label)
        (if _returnvalue
          (goto _label)
          (else
            _)))
      (if _returnvalue_2
        (`self.DestroyWithDamage` (`KismetArrayLibrary.Array_Get` _connectedparts) :!label _label_2)
        (if _returnvalue_2
          (goto _label_2)
          (else
            _)))
      (`self.DetachRootComponentFromParent` true)
      (`PrimitiveComponent.SetSimulatePhysics` (`self.StaticMesh`) true)
      (cast `/Game/Editor/ShipParts/Part_Main` self
        (:`then`
          (`self.K2_DestroyActor` _spaceshipref)
          (`KismetSystemLibrary.PrintString` (`KismetStringLibrary.Concat_StrStr` (`KismetSystemLibrary.GetDisplayName` _spaceshipref) " Detroyed !!!") true true (struct :`R` 1.0 :`G` 0.024691 :`A` 1.0)))
        (:`CastFailed`
          _))
      (`/Engine/EditorBlueprintResources/StandardMacros.IsValid` _parentpart
        (:`Is Valid`
          (`KismetArrayLibrary.Array_RemoveItem` (`/Game/Editor/Blueprints/SelectablePart.ConnectedParts` _parentpart) self))))))

(fn `GetAllSStructs`
  (params (Current :type "/Game/Editor/Blueprints/SelectablePart Object Reference") (GivenID :type Integer :default 0))
  (returns (AllDesignReturned :type "Array of /Game/Editor/Blueprints/StructSelectable Structure") (LastGivenID :type Integer))
  (locals (AllDesign :type "Array of /Game/Editor/Blueprints/StructSelectable Structure") (TempID :type Integer))
  (`/Engine/EditorBlueprintResources/StandardMacros.IsValid` Current
    (:`Is Valid`
      (bind _output_get (set `local.TempID` GivenID))
      (bind _struct (`self.MakeStruct` Current _output_get))
      (`KismetArrayLibrary.Array_Add` (`local.AllDesign`) _struct)
      (for _array_element (`/Game/Editor/Blueprints/SelectablePart.ConnectedModuls` Current)
        (`/Engine/EditorBlueprintResources/StandardMacros.IsValid` _array_element
          (:`Is Valid`
            (bind _output_get_2 (set `local.TempID` (+ (`local.TempID`) 1)))
            (bind _struct_2 (`self.MakeStruct` _array_element _output_get_2))
            (`KismetArrayLibrary.Array_Add` (`local.AllDesign`) _struct_2))))
      (for _array_element_2 (`/Game/Editor/Blueprints/SelectablePart.ConnectedParts` Current)
        (`/Engine/EditorBlueprintResources/StandardMacros.IsValid` _array_element_2
          (:`Is Valid`
            (bind _output_get_3 (set `local.TempID` (+ 1 (`local.TempID`))))
            (bind (_alldesignreturned _lastgivenid) (`self.GetAllSStructs` _array_element_2 _output_get_3))
            (set `local.TempID` _lastgivenid)
            (`KismetArrayLibrary.Array_Append` (`local.AllDesign`) _alldesignreturned))))
      (return (`local.AllDesign`) (`local.TempID`)))
    (:`Is Not Valid`
      (return (`local.AllDesign`) GivenID))))

(fn `isMyChild`
  (params (PossiblyChild :type "/Game/Editor/Blueprints/SelectablePart Object Reference"))
  (returns (isMyChild :type Boolean))
  (for _array_element (`self.ConnectedParts`)
    (if (== _array_element PossiblyChild)
      (return true)))
  (return false))

(fn `MakeSelectable`
  (params (SelectableStruct :type "/Game/Editor/Blueprints/StructSelectable Structure"))
  (returns (Selectablepart :type "/Game/Editor/Blueprints/SelectablePart Object Reference") (ConnectedPartCount :type Integer) (ConnectedModelCount :type Integer))
  (bind (_id _class _location _rotation _scale _mateial _connectedparts _connectedmodules _shapetype _eyeangle) (break `/Game/Editor/Blueprints/StructSelectable` SelectableStruct))
  (bind _returnvalue (`|SpawnActorFromClass` _class (`KismetMathLibrary.MakeTransform` (+ _location (`self.K2_GetActorLocation`)) _rotation _scale) "Undefined" "OverrideRootScale"))
  (bind _output_get (set `/Game/Editor/Blueprints/SelectablePart.ID` _id _returnvalue))
  (`TextRenderComponent.K2_SetText` (`self.TextID`) (`KismetTextLibrary.Conv_IntToText` _output_get))
  (bind _asship_part_bp (cast `/Game/Editor/Blueprints/ShipPartBP` _returnvalue)
    (:`then`
      (set `/Game/Editor/Blueprints/ShipPartBP.ShapeType` _shapetype _asship_part_bp))
    (:`CastFailed`
      _))
  (bind _asship_modul_bp (cast `/Game/Editor/Blueprints/ShipModulBP` _returnvalue)
    (:`then`
      (set `/Game/Editor/Blueprints/ShipModulBP.VisibleAngle` _eyeangle _asship_modul_bp)
      (`/Game/Editor/Blueprints/ShipModulBP.InitAngle` _asship_modul_bp))
    (:`CastFailed`
      _))
  (return _returnvalue (`KismetArrayLibrary.Array_Length` _connectedparts) (`KismetArrayLibrary.Array_Length` _connectedmodules)))

(fn `MakeStruct`
  (params (SelectablePart :type "/Game/Editor/Blueprints/SelectablePart Object Reference") (ID :type Integer))
  (returns (Struct :type "/Game/Editor/Blueprints/StructSelectable Structure"))
  (locals (TempConnectedParts :type "Array of /Game/Editor/Blueprints/SelectablePart Class Reference") (TempConnectedModules :type "Array of /Game/Editor/Blueprints/SelectablePart Class Reference") (TempAngle :type "Float (double-precision)") (TempShapeType :type "/Game/Editor/Shapes/EShapeType Enum" :default "NewEnumerator0"))
  (for _array_element (`/Game/Editor/Blueprints/SelectablePart.ConnectedParts` SelectablePart)
    (`KismetArrayLibrary.Array_Add` (`local.TempConnectedParts`) (`GameplayStatics.GetObjectClass` _array_element)))
  (for _array_element_2 (`/Game/Editor/Blueprints/SelectablePart.ConnectedModuls` SelectablePart)
    (`KismetArrayLibrary.Array_Add` (`local.TempConnectedModules`) (`GameplayStatics.GetObjectClass` _array_element_2)))
  (bind _asship_modul_bp (cast `/Game/Editor/Blueprints/ShipModulBP` SelectablePart)
    (:`then`
      (bind _output_get (set `local.TempAngle` (`/Game/Editor/Blueprints/ShipModulBP.VisibleAngle` _asship_modul_bp)))
      (`KismetSystemLibrary.PrintString` (`KismetStringLibrary.Conv_DoubleToString` _output_get)))
    (:`CastFailed`
      (bind _asship_part_bp (cast `/Game/Editor/Blueprints/ShipPartBP` SelectablePart)
        (:`then`
          (set `local.TempShapeType` (`/Game/Editor/Blueprints/ShipPartBP.ShapeType` _asship_part_bp)))
        (:`CastFailed`
          _))))
  (return (make `/Game/Editor/Blueprints/StructSelectable` ID (`GameplayStatics.GetObjectClass` SelectablePart) (`self.K2_GetActorLocation` SelectablePart) (`self.K2_GetActorRotation` SelectablePart) (`SceneComponent.K2_GetComponentScale` (`/Game/Editor/Blueprints/SelectablePart.StaticMesh` SelectablePart)) null (`local.TempConnectedParts`) (`local.TempConnectedModules`) (`local.TempShapeType`) (`local.TempAngle`))))

(fn `UserConstructionScript`
  (bind _returnvalue (`MaterialInterface.GetBaseMaterial` (`PrimitiveComponent.GetMaterial` (`self.StaticMesh`) 0)))
  (set `self.MaterialDefault` _returnvalue))