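; Blueprint for a ship module that shows its visible angle on an aim-area mesh.
; On BeginPlay it creates a dynamic material instance for that mesh and feeds VisibleAngle into its Percent parameter.
; Simulate calls the parent, then hides the angle mesh while simulation runs and shows it otherwise.
; Activate and Deactivate only toggle the IsActivated flag.
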(event `self.ReceiveBeginPlay`
  (bind _returnvalue (`PrimitiveComponent.CreateDynamicMaterialInstance` (`self.StaticMeshAngle`) 0 "/Game/Editor/Materials/M_AimArea_Inst.M_AimArea_Inst"))
  (`/Engine/EditorBlueprintResources/StandardMacros.IsValid` _returnvalue
    (:`Is Valid`
      (bind _output_get (set `self.MaterialAngle` _returnvalue))
      (`PrimitiveComponent.SetMaterial` (`self.StaticMeshAngle`) 0 _output_get)
      (`self.InitAngle`))))

(event `Activate`
  (set `self.isActivated` true))

(event `Deactivate`
  (set `self.isActivated` false))

(event `self.Simulate`
  (params (isSimulating :type Boolean))
  (`parent.Simulate` isSimulating)
  (`SceneComponent.SetVisibility` (`self.StaticMeshAngle`) (!= (`self.isSimulating`) true) false))

(fn `InitAngle`
  (`MaterialInstanceDynamic.SetScalarParameterValue` (`self.MaterialAngle`) "Percent" (`self.VisibleAngle`)))

(fn `UserConstructionScript`
  (`parent.UserConstructionScript`))