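; Player pawn for the spaceship simulator, giving RTS-style control to spawn, select, move and delete ships.
; On BeginPlay it sets up the selection HUD and simulator widget; number keys pick a save slot that Q spawns at the cursor.
; Drag-selection from SelectHUD feeds right-click move orders to ship AI controllers, with press-drag-release setting facing.
; Actions route through Server events, and SetCamera can snap or attach the pawn to a selected ship.
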(event `Key|Delete`
  (params (Key :type "Key Structure" :default "AnyKey"))
  ;[1 0.12 0.12] Server_DestroyShip
  (:`Pressed`
    (`self.Server_DestroyShip`)))

(event `Server_DestroyShip`
  ;[1 0.12 0.12] Server_DestroyShip
  (for _array_element (`self.SelectedSpaceShips`)
    (`/Game/Editor/NPC/SpaceShipActor.Delete` _array_element)))

(event `self.ReceiveBeginPlay`
  (bind _returnvalue (`GameplayStatics.GetPlayerController` 0))
  ;[1 1 1] Event Begin Play
  (if (not (`KismetSystemLibrary.IsDedicatedServer`))
    (`PlayerController.ClientSetHUD` _returnvalue "/Game/Editor/Widgets/SelectHUD.SelectHUD_C")
    (bind _returnvalue_2 (`|CreateWidget` "/Game/Editor/Widgets/Widget_Sımulator.Widget_Sımulator_C" _returnvalue))
    (bind _output_get (set `self.Widget_Simulator` _returnvalue_2))
    (`UserWidget.AddToViewport` _output_get 0)
    (`UserWidget.AddToViewport` _returnvalue_2 0)
    (bind _asclient_player_controller (cast `/Game/Editor/Blueprints/ClientPlayerController` (`GameplayStatics.GetPlayerController` 0)))
    (set `/Game/Editor/Blueprints/ClientPlayerController.Widget_Simulator` _returnvalue_2 _asclient_player_controller)))

(event `Key|One`
  (params (Key :type "Key Structure" :default "AnyKey"))
  (:`Pressed`
    (set `self.SelectedLoadIndex` 0)))

(event `Server_SpawnShip`
  (params (Transform :type "Transform Structure") (StructSave :type "/Game/Editor/Blueprints/StructSave Structure") (TeamID :type Integer))
  ;[1 0.12 0.12] Server_SpawnShip
  (bind _spaceshipsaveref (`/Game/Editor/Blueprints/MacroLibrary.BreakStructSave` StructSave))
  (bind _newshipcharacter (`self.CreateNewSpaceShipCharacter` _spaceshipsaveref (.location Transform) TeamID))
  (`/Game/Editor/NPC/SpaceShipActor.SetInSimulator` _newshipcharacter true)
  (`self.SetActorRotation` _newshipcharacter (.rotation Transform))
  (bind _returnvalue (`AIBlueprintHelperLibrary.GetAIController` _newshipcharacter))
  (bind _asspace_ship_aicontroller (cast `/Game/Editor/NPC/SpaceShip_AIController` _returnvalue))
  (`/Game/Editor/NPC/SpaceShip_AIController.Order_ModulsGetReady` _asspace_ship_aicontroller)
  (bind _asclient_player_controller (cast `/Game/Editor/Blueprints/ClientPlayerController` (`GameplayStatics.GetPlayerController` 0)))
  (`KismetArrayLibrary.Array_Add` (`/Game/Editor/Blueprints/ClientPlayerController.OwnSpaceShips` _asclient_player_controller) _newshipcharacter))

(event `Key|Two`
  (params (Key :type "Key Structure" :default "AnyKey"))
  (:`Pressed`
    (set `self.SelectedLoadIndex` 1)))

(event `Key|Three`
  (params (Key :type "Key Structure" :default "AnyKey"))
  (:`Pressed`
    (set `self.SelectedLoadIndex` 2)))

(event `Key|Four`
  (params (Key :type "Key Structure" :default "AnyKey"))
  (:`Pressed`
    (set `self.SelectedLoadIndex` 3)))

(event `InputAxisKey|MouseX`
  (params (AxisValue :type "Float (single-precision)"))
  ;[1 1 1] Cursor Coordinates
)

(event `InputAxisKey|MouseY`
  (params (AxisValue :type "Float (single-precision)"))
  ;[1 1 1] Cursor Coordinates
)

(event `Key|Five`
  (params (Key :type "Key Structure" :default "AnyKey"))
  (:`Pressed`
    (set `self.SelectedLoadIndex` 4)))

(event `Key|Six`
  (params (Key :type "Key Structure" :default "AnyKey"))
  (:`Pressed`
    (set `self.SelectedLoadIndex` 5)))

(event `Server_MoveShip`
  (params (NewLocation :type "Vector Structure") (NewRotation :type "Rotator Structure"))
  ;[1 0.12 0.12] Server_MoveUnit
  (for _array_element (`self.SelectedSpaceShips`)
    (`/Engine/EditorBlueprintResources/StandardMacros.IsValid` _array_element
      (:`Is Valid`
        (bind _returnvalue (`AIBlueprintHelperLibrary.GetAIController` _array_element))
        (bind _asspace_ship_aicontroller (cast `/Game/Editor/NPC/SpaceShip_AIController` _returnvalue)
          (:`then`
            (`/Game/Editor/NPC/SpaceShip_AIController.Order_Move` _asspace_ship_aicontroller NewLocation NewRotation))
          (:`CastFailed`
            (`KismetSystemLibrary.PrintString` "AI Cast error"))))
      (:`Is Not Valid`
        (`KismetArrayLibrary.Array_RemoveItem` (`self.SelectedSpaceShips`) _array_element)))))

(event `Key|Seven`
  (params (Key :type "Key Structure" :default "AnyKey"))
  (:`Pressed`
    (set `self.SelectedLoadIndex` 6)))

(event `Key|Eight`
  (params (Key :type "Key Structure" :default "AnyKey"))
  (:`Pressed`
    (set `self.SelectedLoadIndex` 7)))

(event `Key|RightMouseButton`
  (params (Key :type "Key Structure" :default "AnyKey"))
  (bind _templocationmove (`self.TempLocationMove`))
  (bind _returnvalue (`KismetMathLibrary.MakeVector` (.x (`self.CursorRayTraceWithFloor`)) (.y (`self.CursorRayTraceWithFloor`))))
  ;[1 1 1] Move Ship
  (:`Pressed`
    (set `self.TempLocationMove` _returnvalue))
  (:`Released`
    (if (== _returnvalue _templocationmove :`ErrorTolerance` 200.0)
      (`self.Server_MoveShip` (`self.TempLocationMove`))
      (else
        (`self.Server_MoveShip` (`self.TempLocationMove`) (`KismetMathLibrary.FindLookAtRotation` _templocationmove _returnvalue))))))

(event `Key|Nine`
  (params (Key :type "Key Structure" :default "AnyKey"))
  (:`Pressed`
    (set `self.SelectedLoadIndex` 8)))

(event `Server_SelectSpaceShip`
  (params (SelectedActor :type "Array of /Game/Editor/NPC/SpaceShipActor Object Reference"))
  ;[1 0.12 0.12] Server_SelectShip
  (for _array_element (`self.SelectedSpaceShips`)
    (`/Engine/EditorBlueprintResources/StandardMacros.IsValid` _array_element
      (:`Is Valid`
        (`/Game/Editor/NPC/SpaceShipActor.Unselect` _array_element))))
  (bind _output_get (set `self.SelectedSpaceShips` SelectedActor))
  (for _array_element_2 _output_get
    (`/Game/Editor/NPC/SpaceShipActor.Select` _array_element_2)))

(event `Key|Zero`
  (params (Key :type "Key Structure" :default "AnyKey"))
  (:`Pressed`
    (set `self.SelectedLoadIndex` 9)))

(event `Key|Q`
  (params (Key :type "Key Structure" :default "AnyKey"))
  ;[1 1 1] Spawn SpaceShip
  (:`Pressed`
    (set `self.TempLocationSpawn` (`self.CursorRayTraceWithFloor`)))
  (:`Released`
    (bind _asmy_game_instance (cast `/Game/Editor/Maps/MyGameInstance` (`GameplayStatics.GetGameInstance`)))
    (bind _shipsave (`/Game/Editor/Maps/MyGameInstance.GetShipSave` _asmy_game_instance (`self.SelectedLoadIndex`)))
    (`/Engine/EditorBlueprintResources/StandardMacros.IsValid` _shipsave
      (:`Is Valid`
        (bind _structsave (`/Game/Editor/Blueprints/MacroLibrary.MakeStructSave` _shipsave)
          (:`NewParam`
            (`self.Server_SpawnShip` (`KismetMathLibrary.MakeTransform` (`KismetMathLibrary.MakeVector` (.x (`self.TempLocationSpawn`)) (.y (`self.TempLocationSpawn`))) (`KismetMathLibrary.FindLookAtRotation` (`self.TempLocationSpawn`) (`self.CursorRayTraceWithFloor`)) (1.0 1.0 1.0)) _structsave (`self.TEAM`)))))
      (:`Is Not Valid`
        (`KismetSystemLibrary.PrintString` "SaveIndexGecerliDeil")))))

(event `Key|LeftMouseButton`
  (params (Key :type "Key Structure" :default "AnyKey"))
  (bind _returnvalue (`GameplayStatics.GetPlayerController` 0))
  (bind _returnvalue_2 (`PlayerController.GetHUD` _returnvalue))
  (bind (_locationx _locationy) (`PlayerController.GetMousePosition` _returnvalue))
  ;[1 1 1] Order Move
  (:`Pressed`
    (bind _asselect_hud (cast `/Game/Editor/Widgets/SelectHUD` _returnvalue_2))
    (set `/Game/Editor/Widgets/SelectHUD.FirstPoint` (`KismetMathLibrary.MakeVector2D` _locationx _locationy) _asselect_hud)
    (set `/Game/Editor/Widgets/SelectHUD.isSelecting` true _asselect_hud))
  (:`Released`
    (bind _asselect_hud_2 (cast `/Game/Editor/Widgets/SelectHUD` _returnvalue_2))
    (bind _selectedspaceships (`/Game/Editor/Widgets/SelectHUD.SelectedSpaceShips` _asselect_hud_2))
    (`self.Server_SelectSpaceShip` _selectedspaceships)
    (`KismetSystemLibrary.PrintString` (`KismetStringLibrary.BuildString_Int` "" "" (`KismetArrayLibrary.Array_Length` _selectedspaceships) " Gemi Secildi"))
    (set `/Game/Editor/Widgets/SelectHUD.isSelecting` false _asselect_hud_2)))

(fn `SetCamera`
  (params (CamNo :type Integer))
  (bind _returnvalue (`GameplayStatics.GetPlayerPawn` 0))
  (bind _returnvalue_2 (`GameplayStatics.GetPlayerPawn` 0))
  (bind _selectedspaceships (`self.SelectedSpaceShips`))
  (bind _item (`KismetArrayLibrary.Array_Get` (`self.SelectedSpaceShips`)))
  (bind _item_2 (`KismetArrayLibrary.Array_Get` (`self.SelectedSpaceShips`)))
  (`self.DetachRootComponentFromParent` self true)
  (if (< (`KismetArrayLibrary.Array_Length` _selectedspaceships) 2)
    (`/Engine/EditorBlueprintResources/StandardMacros.IsValid` (`KismetArrayLibrary.Array_Get` _selectedspaceships)
      (:`Is Valid`
        (switch `int` CamNo
          (:`0`
            (`self.K2_SetActorLocation` _returnvalue (`self.K2_GetActorLocation` _item) false false)
            (`self.SetActorRotation` _returnvalue (`self.K2_GetActorRotation` _item))
            (`SceneComponent.K2_AttachTo` (`self.CollisionComponent`) (`/Game/Editor/NPC/SpaceShipActor.StaticMesh` (`KismetArrayLibrary.Array_Get` (`self.SelectedSpaceShips`))) "None" "KeepWorldPosition" true)
            (`self.SetActorRotation` self (`self.K2_GetActorRotation`)))
          (:`1`
            (`SceneComponent.K2_AttachTo` (`self.CollisionComponent`) (`/Game/Editor/NPC/SpaceShipActor.StaticMesh` (`KismetArrayLibrary.Array_Get` (`self.SelectedSpaceShips`))) "None" "KeepWorldPosition" true))
          (:`2`
            (`self.K2_SetActorLocation` _returnvalue_2 (`self.K2_GetActorLocation` _item_2) false false)
            (`self.SetActorRotation` _returnvalue_2 (`self.K2_GetActorRotation` _item_2))
            (`PlayerController.SetViewTargetWithBlend` (`GameplayStatics.GetPlayerController` 0) _returnvalue_2 0.0 "VTBlend_Linear" 0.0 true)))))
    (else
      (`KismetSystemLibrary.PrintString` "Tek Adam Secilmeli"))))

(fn `UserConstructionScript`
  (`parent.UserConstructionScript`))