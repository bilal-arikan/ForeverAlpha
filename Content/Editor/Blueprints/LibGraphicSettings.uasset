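; Function library of graphics setters that change display and quality settings at runtime.
; Each function builds a console command string from its input and executes it through player controller 0.
; It covers fullscreen mode, resolution and screen percentage, anti-aliasing, view distance, and scalability groups for effects, shadows, textures and post-processing.
; Only the resolution setter validates input, requiring positive dimensions, and it always appends the fullscreen suffix.
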(fn `SetAntiAlliasign`
  (params (`Level (0-6)` :type Integer))
  (`KismetSystemLibrary.ExecuteConsoleCommand` null (`KismetStringLibrary.Concat_StrStr` "r.PostProcessAAQuality " (`KismetStringLibrary.Conv_IntToString` `Level (0-6)`)) (`GameplayStatics.GetPlayerController` null))
  (return))

(fn `SetEffect`
  (params (`Level (0-3)` :type Integer))
  (`KismetSystemLibrary.ExecuteConsoleCommand` null (`KismetStringLibrary.Concat_StrStr` "sg.EffectsQuality " (`KismetStringLibrary.Conv_IntToString` `Level (0-3)`)) (`GameplayStatics.GetPlayerController` null))
  (return))

(fn `SetFullscreen`
  (params (isFull :type Boolean))
  (`KismetSystemLibrary.ExecuteConsoleCommand` null (`KismetMathLibrary.SelectString` "r.fullscreenmode 0" "r.fullscreenmode 1" isFull) (`GameplayStatics.GetPlayerController` null))
  (return))

(fn `SetPostProcess`
  (params (`Level (0-3)` :type Integer))
  (`KismetSystemLibrary.ExecuteConsoleCommand` null (`KismetStringLibrary.Concat_StrStr` "sg.PostProcessQuality " (`KismetStringLibrary.Conv_IntToString` `Level (0-3)`)) (`GameplayStatics.GetPlayerController` null))
  (return))

(fn `SetResolution`
  (params (X :type Integer) (Y :type Integer))
  (if (and (> X 0) (> Y 0))
    (`KismetSystemLibrary.ExecuteConsoleCommand` null (`KismetStringLibrary.Concat_StrStr` "r.setRes " (`KismetStringLibrary.Conv_IntToString` X) "x" (`KismetStringLibrary.Conv_IntToString` Y) "f") (`GameplayStatics.GetPlayerController` null))))

(fn `SetResolutionScale`
  (params (Percent :type Integer))
  (`KismetSystemLibrary.ExecuteConsoleCommand` null (`KismetStringLibrary.Concat_StrStr` "r.ScreenPercentage " (`KismetStringLibrary.Conv_IntToString` Percent)) (`GameplayStatics.GetPlayerController` null))
  (return))

(fn `SetShadow`
  (params (`level (0-3)` :type Integer))
  (`KismetSystemLibrary.ExecuteConsoleCommand` null (`KismetStringLibrary.Concat_StrStr` "sg.ShadowQuality " (`KismetStringLibrary.Conv_IntToString` `level (0-3)`)) (`GameplayStatics.GetPlayerController` null))
  (return))

(fn `SetTexture`
  (params (Level :type Integer))
  (`KismetSystemLibrary.ExecuteConsoleCommand` null (`KismetStringLibrary.Concat_StrStr` "sg.TextureQuality " (`KismetStringLibrary.Conv_IntToString` Level)) (`GameplayStatics.GetPlayerController` null))
  (return))

(fn `SetViewDistance`
  (params (`Distance (0-1)` :type "Float (double-precision)"))
  (`KismetSystemLibrary.ExecuteConsoleCommand` null (`KismetStringLibrary.Concat_StrStr` "r.ViewDistanceScale " (`KismetStringLibrary.Conv_DoubleToString` `Distance (0-1)`)) (`GameplayStatics.GetPlayerController` null))
  (return))