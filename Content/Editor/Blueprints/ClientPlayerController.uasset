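; Player controller for a captain-based simulator game, handling spawn requests, team assignment and the escape menu.
; ClientPostLogin asks SimulatorGameMode to spawn a captain for this controller, printing an error if the cast fails.
; SetTeam stores the team number and copies it to the possessed CharacterCaptain.
; BeginPlay creates the escape and options widgets; the Quote key toggles the escape menu, while options is only stored here.
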(event `SetTeam`
  (params (number :type Integer))
  (set `self.TEAM` number)
  (bind _ascharacter_captain (cast `/Game/Editor/Blueprints/CharacterCaptain` (`self.K2_GetPawn`)))
  (set `/Game/Editor/Blueprints/CharacterDefault.TEAM` number _ascharacter_captain))

(event `ClientPostLogin`
  (bind _assimulator_game_mode (cast `/Game/Editor/Maps/SimulatorGameMode` (`GameplayStatics.GetGameMode`))
    (:`then`
      (`/Game/Editor/Maps/SimulatorGameMode.SpawnNewCaptain` _assimulator_game_mode self))
    (:`CastFailed`
      (`KismetSystemLibrary.PrintString` "(Client) Gamemode Cast Error "))))

(event `Key|Quote`
  (params (Key :type "Key Structure" :default "AnyKey"))
  (bind _w_esc (`self.W_ESC`))
  (:`Pressed`
    (`/Engine/EditorBlueprintResources/StandardMacros.FlipFlop`
      (:`A`
        (`UserWidget.AddToViewport` _w_esc 0))
      (:`B`
        (`Widget.RemoveFromParent` _w_esc)))))

(event `self.ReceiveBeginPlay`
  (bind _returnvalue (`|CreateWidget` "/Game/Editor/Widgets/W_ESC.W_ESC_C"))
  (set `self.W_ESC` _returnvalue)
  (bind _returnvalue_2 (`|CreateWidget` "/Game/Editor/Widgets/W_Options.W_Options_C" null _returnvalue))
  (set `self.W_Options` _returnvalue_2))

(event `self.ReceiveTick`
  (params (DeltaSeconds :type "Float (single-precision)")))

(fn `UserConstructionScript`)